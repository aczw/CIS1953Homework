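; BPC_ProjectileShooter is a component that fires physics-driven BP_Projectile balls along a camera's forward vector, limited by a charge count.
; Charges fill to the maximum on BeginPlay, with clamped increment and decrement functions that print debug messages.
; Shoot spawns the ball ahead of the given actor, ignores that actor during movement, applies an impulse and spends a charge.
; Each shot also starts a looping timer whose bound event is not shown.
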(event EventBeginPlay
  (bind _output_get (Variables|Default|SetNum%20Charges (Variables|Default|GetMaximum%20Charges)))
  (Development|PrintString (Utilities|String|BuildString(Integer) "" "[Debug] Set Num Charges to " _output_get)))

(fn IncrementNumCharges
  (if (< (Variables|Default|GetNum%20Charges) (Variables|Default|GetMaximum%20Charges))
    (bind _result (Math|Integer|IncrementInt (Variables|Default|GetNum%20Charges))
      (:%20%20
        (Development|PrintString (Utilities|String|BuildString(Integer) "" "[Debug] Incremented Num Charges to " _result))))))

(fn DecrementNumCharges
  (if (> (Variables|Default|GetNum%20Charges) 0)
    (bind _result (Math|Integer|DecrementInt (Variables|Default|GetNum%20Charges))
      (:%20%20
        (Development|PrintString (Utilities|String|BuildString(Integer) "" "[Debug] Decremented Num Charges to " _result))))))

(fn Shoot
  (params (Actor%20Camera :type Camera%20Component%20Object%20Reference%20%28by%20ref%29) (Actor :type Actor%20Object%20Reference%20%28by%20ref%29))
  (bind _returnvalue (Math|Vector|GetForwardVector Actor%20Camera))
  (if (> (Variables|Default|GetNum%20Charges) 0)
    (bind _returnvalue_2 (Game|SpawnActorfromClass "/Game/Blueprints/BP_Projectile.BP_Projectile_C" (Math|Transform|MakeTransform (+ (* _returnvalue 55.0) (Transformation|GetActorLocation Actor) "0.000000,0.000000,40.000000")) "AlwaysSpawn" "MultiplyWithRoot" 0 0))
    (Collision|IgnoreActorwhenMoving (Variables|/Game/Blueprints/BP_Projectile.BP_Projectile_C|GetBall _returnvalue_2) Actor true)
    (Physics|AddImpulse (Variables|/Game/Blueprints/BP_Projectile.BP_Projectile_C|GetBall _returnvalue_2) (* _returnvalue 1e+04) "None" false)
    (CallFunction|DecrementNumCharges)
    (Utilities|Time|SetTimerbyEvent (EventDispatchers|CreateEvent :!event IncrementNumCharges) 2.0 true)))