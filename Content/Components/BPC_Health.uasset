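; Health component that tracks an actor's current and maximum hit points.
; Current starts at Maximum on BeginPlay, and GainHealth adds an amount clamped between zero and Maximum.
; LoseHealth subtracts damage and, at zero or below, sets Current to zero and calls OnDeathMessage on the owner.
; Each change prints a debug string to the screen.
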(event EventBeginPlay
  (bind _output_get (Variables|Default|SetCurrent (Variables|Default|GetMaximum)))
  (Development|PrintString (Utilities|String|BuildString(Integer) "" "[Debug] Set health to " _output_get)))

(fn GainHealth
  (params (Amount :type Integer))
  (Variables|Default|SetCurrent (Math|Integer|Clamp(Integer) (+ Amount (Variables|Default|GetCurrent)) 0 (Variables|Default|GetMaximum)))
  (Development|PrintString (Utilities|String|BuildString(Integer) "" "[Debug] Gained " Amount " health")))

(fn LoseHealth
  (params (Amount :type Integer))
  (bind _returnvalue (Components|GetOwner))
  (if (<= (- (Variables|Default|GetCurrent) Amount) 0)
    (Variables|Default|SetCurrent 0)
    (Development|PrintString "[Debug] Died!")
    (Class|BICharacter|OnDeath(Message) _returnvalue)
    (else
      (Variables|Default|SetCurrent (- (Variables|Default|GetCurrent) Amount))
      (Development|PrintString (Utilities|String|BuildString(Integer) (Utilities|String|BuildString(Integer) "" (Utilities|String|Append "[Debug] [" (Utilities|GetDisplayName _returnvalue) "] Lost ") Amount " health: ") "now " (Variables|Default|GetCurrent) " HP!")))))