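; BP_TargetSpawner spawns a batch of target actors and can destroy them on demand.
; SpawnTargets creates SpawnCount actors of the Target class at SpawnOrigin, ignoring collision, passing each a fixed SpawnRange vector and storing it in SpawnedTargets.
; DestroyTargets destroys every still-valid actor in that array without clearing it.
; Neither function is called within this Blueprint, and the construction script is empty.
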(fn ConstructionScript)

(fn SpawnTargets
  (for _index (range 1 (Variables|Default|GetSpawn%20Count))
    (bind _returnvalue (Game|SpawnActorfromClass (Variables|Default|GetTarget) (Math|Transform|MakeTransform (Variables|Default|GetSpawn%20Origin)) "AlwaysSpawn" "MultiplyWithRoot" 0 "500.000000,600.000000,300.000000" 0))
    (Utilities|Array|Add (Variables|Default|GetSpawned%20Targets) _returnvalue)))

(fn DestroyTargets
  (for _array_element (Variables|Default|GetSpawned%20Targets)
    (Utilities|IsValid _array_element
      (:Is%20Valid
        (Actor|DestroyActor _array_element)))))