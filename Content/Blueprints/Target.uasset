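; Target actor that jumps to a random location within a box around its starting position.
; On BeginPlay it stores the root component's location as Origin, then picks a random point within SpawnRange centred on it, per axis.
; A Cylinder hit repeats the move only when the other actor is not valid, so hits from valid actors leave it in place.
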(event OnComponentHit(Cylinder)
  (params (HitComponent :type Primitive%20Component%20Object%20Reference) (OtherActor :type Actor%20Object%20Reference) (OtherComp :type Primitive%20Component%20Object%20Reference) (NormalImpulse :type Vector :default "0, 0, 0") (Hit :type Hit%20Result%20Structure%20%28by%20ref%29))
  (Utilities|IsValid OtherActor
    (:Is%20Not%20Valid
      (CallFunction|MovetoRandomLocation))))

(event EventBeginPlay
  (Variables|Default|SetOrigin (Variables|/Script/Engine.SceneComponent|GetRelativeLocation (Variables|Default|GetDefaultSceneRoot)))
  (CallFunction|MovetoRandomLocation))

(fn ConstructionScript)

(fn MovetoRandomLocation
  (bind _spawn_range (Variables|Default|GetSpawn%20Range))
  (bind _origin (Variables|Default|GetOrigin))
  (bind _returnvalue (* _spawn_range 0.5))
  (bind _returnvalue_2 (Math|Vector|NegateVector _returnvalue))
  (bind _returnvalue_3 (+ _returnvalue _origin))
  (bind (_x _y _z) (Math|Vector|BreakVector _returnvalue_3))
  (bind _returnvalue_4 (+ _origin _returnvalue_2))
  (bind (_x_2 _y_2 _z_2) (Math|Vector|BreakVector _returnvalue_4))
  (Transformation|SetActorLocation (Math|Vector|MakeVector (Math|Random|RandomFloatinRange _x_2 _x) (Math|Random|RandomFloatinRange _y_2 _y) (Math|Random|RandomFloatinRange _z_2 _z)) false false))